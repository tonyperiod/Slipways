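; Scene component that detects whether it is over a lava surface within trace range.
; Every tick it line-traces along its negative up vector by TraceLength and sets TouchingLava when the hit physical material matches Lava.
; It only maintains that flag, applying no effects itself, and leaves timed debug drawing of the trace enabled.
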(event `self.ReceiveTick`
  (params (DeltaSeconds :type "Float (single-precision)"))
  (bind _returnvalue (`self.K2_GetComponentLocation`))
  (bind _outhit (`KismetSystemLibrary.LineTraceSingle` :`Start` _returnvalue :`End` (+ _returnvalue (* (`self.GetUpVector`) (* (`self.Trace Length`) -1.0))) :`TraceChannel` "TraceTypeQuery3" :`DrawDebugType` "ForDuration" :`DrawTime` 0.01))
  (set `self.Touching Lava` (== (`.PhysMat` (`GameplayStatics.BreakHitResult` _outhit)) (`self.Lava`))))