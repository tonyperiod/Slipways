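; Component that tracks a signed forward/reverse Acceleration value for the player's Cube from Move Forward / Backward axis input.
; Tick and the axis event share one update that accumulates within the max limit, decelerates otherwise, boosts opposite-direction input and snaps near-zero values to zero.
; CalculateFOV linearly widens the camera FOV as forward acceleration rises above a threshold.
; Movement is not applied here; getters and setters expose the value and tuning.
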(event `Init Component`
  (params (Cube :type "StaticMeshComponent Object Reference") (Camera :type "CameraComponent Object Reference") (`Touching Lava` :type Boolean))
  ;[1 0 0.7773] Initializer
  (set `self.Camera` Camera)
  (set `self.Cube` Cube)
  (set `self.Acceleration` 0.0))

(event `self.ReceiveTick`
  (params (DeltaSeconds :type "Float (single-precision)"))
  (bind _returnvalue (> (stale `InputAxis|Move Forward / Backward` AxisValue) 0.0))
  (set `self.Moving Forward` _returnvalue :!label _label)
  (`self.Calculate FOV`)
  ;[0.07239 0.9702 1] If Player is Holding W or S
  (if (or _returnvalue (< (stale `InputAxis|Move Forward / Backward` AxisValue) 0.0))
    ;[1 0.8899 0.2708] Checks if below max speed
    (if (and (< (`self.Acceleration`) (`self.Max Acceleration`)) (> (`self.Acceleration`) (* (`self.Max Acceleration`) -1.0)))
      ;[0.3582 1 0.4198] If Player is Moving Forward or Backwards (based on Keyboard Input)
      (if (`self.Moving Forward`)
        (`self.Increase Acceleration` (`self.Forward Acceleration`))
        ;[1 0.2497 0.2696] If Pressing W and moving Backwards
        (if (< (`self.Acceleration`) 0.0)
          (`self.Decrease Acceleration` (`self.Deceleration`)))
        (else
          (`self.Increase Acceleration` (`self.Reverse Acceleration`) true)
          ;[1 0.2497 0.2696] If Pressing S and moving Forwards
          (if (>= (`self.Acceleration`) 0.0)
            (`self.Decrease Acceleration` (`self.Deceleration`)) ; Decelerates if going opposite direction to current velocity
          )))
      (else
        (`self.Decrease Acceleration` (`self.Deceleration`))))
    (else
      ;[1 0.2993 0.3591] If not pressing either key
      (`self.Decrease Acceleration` (`self.Deceleration`)))))

(event `InputAxis|Move Forward / Backward`
  (params (AxisValue :type "Float (single-precision)"))
  ;[1 1 1] If player is trying to move forwards or backwards
  (goto _label))

(fn `Calculate FOV`
  (bind _camera (`self.Camera`))
  (bind _begin_fov_acceleration (`self.Begin FOV Acceleration`))
  (if (> (`self.Acceleration`) (`self.Max Acceleration`))
    (`CameraComponent.SetFieldOfView` (`self.Camera`) (`self.Max FOV`))
    (elif (> (`self.Acceleration`) (`self.Begin FOV Acceleration`))
      (`CameraComponent.SetFieldOfView` _camera (+ (* (* (/ (- (`self.Acceleration`) _begin_fov_acceleration) (- (`self.Max Acceleration`) _begin_fov_acceleration)) 100.0) (/ (- (`self.Max FOV`) (`self.Min FOV`)) 100.0)) (`self.Min FOV`)))
      (else
        (`CameraComponent.SetFieldOfView` _camera (`self.Min FOV`))))))

(fn `Decrease Acceleration`
  (params (`Decrease Value` :type "Float (double-precision)"))
  (locals (`Increment Value` :type "Float (double-precision)"))
  (bind _acceleration (`self.Acceleration`))
  ;[1 1 1] Sets Decrease Value for use later
  (set `local.Increment Value` `Decrease Value`)
  ;[1 0.3548 0.349] Sets Acceleration to 0 (If close enough to 0)
  (if (and (>= _acceleration -50.0) (<= _acceleration 50.0))
    (set `self.Acceleration` 0.0)
    (else
      ;[0.349 1 0.4385] Sets the appropriate direction to decrease acceleration
      (if (> (`self.Acceleration`) 0.0)
        (`self.Increase Acceleration` (`local.Increment Value`) true)
        (else
          (`self.Increase Acceleration` (`local.Increment Value`)))))))

(fn `Get Acceleration`
  (returns (Acceleration :type "Float (double-precision)"))
  (return (`self.Acceleration`)))

(fn `Increase Acceleration`
  (params (`Increase Value` :type "Float (double-precision)") (Reverse :type Boolean))
  (locals (ReverseLocal :type Boolean) (IncrementLocal :type "Float (double-precision)"))
  (bind _incrementlocal (`local.IncrementLocal`))
  (bind _incrementlocal_2 (`local.IncrementLocal`))
  (set `local.IncrementLocal` `Increase Value`)
  (set `local.ReverseLocal` Reverse)
  (if (or (and (`local.ReverseLocal`) (> (`self.Acceleration`) 0.0)) (and (`self.Moving Forward`) (< (`self.Acceleration`) 0.0)))
    ;[0.1476 1 0.269] Applies Opposite Multiplier
    (if (`local.ReverseLocal`)
      (set `self.Acceleration` (- (`self.Acceleration`) (* (`self.Opposite Multiplier`) _incrementlocal)))
      (else
        (set `self.Acceleration` (+ (* _incrementlocal (`self.Opposite Multiplier`)) (`self.Acceleration`)))))
    (else
      ;[0.2868 0.9202 1] Ignores Multiplier
      (if (`local.ReverseLocal`)
        (set `self.Acceleration` (- (`self.Acceleration`) _incrementlocal_2))
        (else
          (set `self.Acceleration` (+ _incrementlocal_2 (`self.Acceleration`))))))))

(fn `NewFunction_0`)

(fn `Set Acceleration`
  (params (Value :type "Float (double-precision)"))
  (set `self.Acceleration` Value))

(fn `Set Deceleration`
  (params (Value :type "Float (double-precision)"))
  (set `self.Deceleration` Value))

(fn `Set Max Acceleration`
  (params (MaxAcceleration :type "Float (double-precision)"))
  (set `self.Max Acceleration` MaxAcceleration))

(fn `Set Max FOV`
  (params (Value :type "Float (double-precision)"))
  (set `self.Max FOV` Value))

(fn `Set Touching Lava`
  (set `self.Touching Lava` true))