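; SmoothCornerRaycast is an unfinished hoverboard helper component, apparently a prototype for raycast-driven corner smoothing.
; InitComponent casts the passed reference to HoverboardComponent and caches its Cube.
; Tick does nothing; the downward debug line trace along the component's up vector, which prints hit distance, is disconnected.
; Two experimental Cube pitch nudges, in world and local space, are also unwired, so nothing rotates at runtime.
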(event `InitComponent`
  (params (HoverboardReference :type "/Game/A_ProgrammerCommon/Blueprints/HoverboardComponent Object Reference"))
  (bind _output_get (set `self.Hoverboard Reference` HoverboardReference))
  (bind _ashoverboard_component (cast `/Game/A_ProgrammerCommon/Blueprints/HoverboardComponent` _output_get))
  (set `self.Cube` (`/Game/A_ProgrammerCommon/Blueprints/HoverboardComponent.Cube` _ashoverboard_component)))

(event `self.ReceiveTick`
  (params (DeltaSeconds :type "Float (single-precision)")))