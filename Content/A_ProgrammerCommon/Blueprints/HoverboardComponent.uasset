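; Player-steered physics hoverboard that sets up four hover components plus jump, acceleration and in-air components on its Cube mesh.
; Each tick it pushes forward by AccelerationComponent's value and applies constant downward fake gravity.
; Steering yaws both the mesh and its velocity, while the forward/backward axis does nothing.
; Any hover component detecting ground counts as grounded, which feeds InAirComponent along with sphere overlaps.
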(event `InputAction|Jump`
  (params (Key :type "Key Structure"))
  ;[0 0.08256 0.6979] Unused Code (Jumping)
)

(event `self.ReceiveBeginPlay`
  ;[1 1 1] Initializes the Hover Components using the Board's Mesh
  (`/Game/A_ProgrammerCommon/Blueprints/HoverComponent.InitComponent` (`self.HoverComponent`) (`self.Cube`) (`self.hoverForce`))
  (`/Game/A_ProgrammerCommon/Blueprints/HoverComponent.InitComponent` (`self.HoverComponent1`) (`self.Cube`) (`self.hoverForce`))
  (`/Game/A_ProgrammerCommon/Blueprints/HoverComponent.InitComponent` (`self.HoverComponent2`) (`self.Cube`) (`self.hoverForce`))
  (`/Game/A_ProgrammerCommon/Blueprints/HoverComponent.InitComponent` (`self.HoverComponent3`) (`self.Cube`) (`self.hoverForce`))
  (`/Game/Micheal/Blueprints/JumpComponent.Init Component` (`self.JumpComponent`) (`self.Cube`) (`self.jumpForce`))
  (`/Game/Micheal/Blueprints/AccelerationComponent.Init Component` (`self.AccelerationComponent`) (`self.Cube`))
  (`/Game/Ross/Blueprints/InAirComponent.Init Component` (`self.InAirComponent`) (`self.Cube`) (`self.Sphere`)))

(event `InputAxis|Move Forward / Backward`
  (params (AxisValue :type "Float (single-precision)"))
  ;[1 1 1] Backwards and Forwards Movement
  ;;[1 0 0.6288] Local gravity while moving to smooth track movement
  (bind _grounddetected (`self.GroundCheck`))
  (if _grounddetected
    _))

(event `InputAxis|Move Right / Left`
  (params (AxisValue :type "Float (single-precision)"))
  (bind _returnvalue (`KismetMathLibrary.MakeRotator` 0.0 0.0 (* AxisValue (`self.rotationValue`))))
  ;[1 1 1] Left and Right Movement
  (bind _returnvalue_2 (`PrimitiveComponent.GetPhysicsLinearVelocity` (`self.Cube`) "None"))
  (`PrimitiveComponent.SetPhysicsLinearVelocity` (`self.Cube`) (`KismetMathLibrary.GreaterGreater_VectorRotator` _returnvalue_2 _returnvalue) false "None")
  (`SceneComponent.K2_AddLocalRotation` (`self.Cube`) _returnvalue false false))

(event `self.ReceiveTick`
  (params (DeltaSeconds :type "Float (single-precision)"))
  ;[1 1 1] Check the speed and slow down the Hoverboard when not touching ground
  ;;[1 0.06198 0.09183] Additions
  (bind _acceleration (`/Game/Micheal/Blueprints/AccelerationComponent.Get Acceleration` (`self.AccelerationComponent`)))
  (`PrimitiveComponent.AddForce` (`self.Cube`) (* (* _acceleration 1.0) (`SceneComponent.GetForwardVector` (`self.Cube`))) "None" true)
  (bind _acceleration_2 (`/Game/Micheal/Blueprints/AccelerationComponent.Get Acceleration` (`self.AccelerationComponent`)))
  ;;[0.1696 1 0.07667] Check Acceleration
  (`KismetSystemLibrary.PrintString` (`KismetStringLibrary.Conv_DoubleToString` _acceleration_2))
  (bind _grounddetected (`self.GroundCheck`))
  (`/Game/Ross/Blueprints/InAirComponent.OnGround` (`self.InAirComponent`) _grounddetected)
  ;[1 0.3682 0.07432] Fake Gravity so it works better on Tony's Spline (Need to Redo This)
  (if _grounddetected
    _
    (else
      _))
  (`PrimitiveComponent.AddForce` (`self.Cube`) (* (`KismetMathLibrary.GetUpVector` (struct)) -1.0 3000.0) "None" true))

(event `self.Sphere.OnComponentBeginOverlap`
  (params (OverlappedComponent :type "PrimitiveComponent Object Reference") (OtherActor :type "Actor Object Reference") (OtherComp :type "PrimitiveComponent Object Reference") (OtherBodyIndex :type Integer) (bFromSweep :type Boolean) (SweepResult :type "HitResult Structure (by ref)"))
  (`/Game/Ross/Blueprints/InAirComponent.On Overlap` (`self.InAirComponent`)))

(event `self.Sphere.OnComponentEndOverlap`
  (params (OverlappedComponent :type "PrimitiveComponent Object Reference") (OtherActor :type "Actor Object Reference") (OtherComp :type "PrimitiveComponent Object Reference") (OtherBodyIndex :type Integer))
  (`/Game/Ross/Blueprints/InAirComponent.End Overlap` (`self.InAirComponent`)))

(fn `GroundCheck`
  (returns (GroundDetected :type Boolean))
  (return (or (`/Game/A_ProgrammerCommon/Blueprints/HoverComponent.DetectGround` (`self.HoverComponent`)) (`/Game/A_ProgrammerCommon/Blueprints/HoverComponent.DetectGround` (`self.HoverComponent1`)) (`/Game/A_ProgrammerCommon/Blueprints/HoverComponent.DetectGround` (`self.HoverComponent2`)) (`/Game/A_ProgrammerCommon/Blueprints/HoverComponent.DetectGround` (`self.HoverComponent3`)))))

(fn `UserConstructionScript`)