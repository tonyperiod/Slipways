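; Physics-driven hoverboard that the player steers with forward/backward and left/right axis input.
; Four hover components are initialized on the board mesh, and GroundCheck reports grounded if any of them detects ground.
; Throttle pushes along the board's forward vector, flattened horizontally when airborne, while Tick adds downward force off the ground.
; Steering applies yaw torque scaled by the up vector, inverted while S is held.
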(event `self.ReceiveBeginPlay`
  (`/Game/Ross/Blueprints/HoverComponentBP.InitComponent` (`self.HoverComponentBP`) (`self.BoardMesh`))
  (`/Game/Ross/Blueprints/HoverComponentBP.InitComponent` (`self.HoverComponentBP1`) (`self.BoardMesh`))
  (`/Game/Ross/Blueprints/HoverComponentBP.InitComponent` (`self.HoverComponentBP2`) (`self.BoardMesh`))
  (`/Game/Ross/Blueprints/HoverComponentBP.InitComponent` (`self.HoverComponentBP3`) (`self.BoardMesh`)))

(event `InputAxis|Move Forward / Backward`
  (params (AxisValue :type "Float (single-precision)"))
  (bind (_returnvalue_x _returnvalue_y) (`KismetMathLibrary.BreakVector` (`SceneComponent.GetForwardVector` (`self.boardMesh`))))
  (bind _grounddetected (`self.GroundCheck`))
  (if _grounddetected
    (`PrimitiveComponent.AddForce` (`self.boardMesh`) (* (* (`SceneComponent.GetForwardVector` (`self.boardMesh`)) 500000.0) AxisValue) "None" false)
    (else
      (`PrimitiveComponent.AddForce` (`self.boardMesh`) (* (* (`KismetMathLibrary.MakeVector` _returnvalue_x _returnvalue_y) 500000.0) AxisValue) "None" false))))

(event `InputAxis|Move Right / Left`
  (params (AxisValue :type "Float (single-precision)"))
  (`PrimitiveComponent.AddTorqueInDegrees` (`self.boardMesh`) (* (`KismetMathLibrary.MakeVector` 0.0 0.0 (* (`KismetMathLibrary.SelectFloat` -1.0 1.0 (`PlayerController.IsInputKeyDown` (`GameplayStatics.GetPlayerController` 0) "S")) (* AxisValue 80000000.0))) (`SceneComponent.GetUpVector` (`self.boardMesh`))) "None" false))

(event `self.ReceiveTick`
  (params (DeltaSeconds :type "Float (single-precision)"))
  (bind _grounddetected (`self.GroundCheck`))
  (if (not _grounddetected)
    (`PrimitiveComponent.AddForce` (`self.boardMesh`) (0.0 0.0 -50000.0) "None" false)))

(fn `GroundCheck`
  (returns (GroundDetected :type Boolean))
  (return (or (`/Game/Ross/Blueprints/HoverComponentBP.DetectGround` (`self.HoverComponentBP`)) (`/Game/Ross/Blueprints/HoverComponentBP.DetectGround` (`self.HoverComponentBP1`)) (`/Game/Ross/Blueprints/HoverComponentBP.DetectGround` (`self.HoverComponentBP2`)) (`/Game/Ross/Blueprints/HoverComponentBP.DetectGround` (`self.HoverComponentBP3`)))))

(fn `UserConstructionScript`)