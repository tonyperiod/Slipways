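; Component that gives an airborne physics cube gravity and player rotation control.
; InitComponent stores the cube reference, and OnGround sets the TouchingGround flag that gates all behavior.
; While off the ground, Tick applies a constant downward acceleration as a mass-independent force, and the Roll, Pitch and Yaw axes add scaled local rotation.
; The overlap functions are empty stubs.
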(event `Init Component`
  (params (Cube :type "StaticMeshComponent Object Reference") (`Sphere Collider` :type "SphereComponent Object Reference"))
  (set `self.Cube` Cube))

(event `self.ReceiveTick`
  (params (DeltaSeconds :type "Float (single-precision)"))
  (if (not (`self.TouchingGround`))
    (`PrimitiveComponent.AddForce` (`self.Cube`) (0.0 0.0 -1000.0) "None" true)))

(event `InputAxis|Roll`
  (params (AxisValue :type "Float (single-precision)"))
  (if (not (`self.TouchingGround`))
    (`self.K2_AddLocalRotation` (`self.Cube`) (`KismetMathLibrary.MakeRotator` (* (`self.RollFactor`) AxisValue)) false false)))

(event `InputAxis|Pitch`
  (params (AxisValue :type "Float (single-precision)"))
  (if (not (`self.TouchingGround`))
    (`self.K2_AddLocalRotation` (`self.Cube`) (`KismetMathLibrary.MakeRotator` 0.0 (* (`self.PitchFactor`) AxisValue)) false false)))

(event `InputAxis|Yaw`
  (params (AxisValue :type "Float (single-precision)"))
  (if (not (`self.TouchingGround`))
    (`self.K2_AddLocalRotation` (`self.Cube`) (`KismetMathLibrary.MakeRotator` 0.0 0.0 (* (`self.YawFactor`) AxisValue)) false false)))

(fn `End Overlap`)

(fn `On Overlap`)

(fn `OnGround`
  (params (OnGround :type Boolean))
  (set `self.TouchingGround` OnGround))