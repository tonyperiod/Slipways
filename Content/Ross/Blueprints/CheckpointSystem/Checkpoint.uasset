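; Checkpoint actor that detects the hoverboard passing through it in the intended direction.
; On trigger overlap, it casts to HoverboardComponent and takes the dot product of the board cube's velocity and the Arrow's forward vector to reject wrong-way entries.
; A valid pass calls the CheckpointCleared dispatcher with its checkpoint number, hides the trigger and particles, and disables further overlap events.
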(event `self.Trigger.OnComponentBeginOverlap`
  (params (OverlappedComponent :type "PrimitiveComponent Object Reference") (OtherActor :type "Actor Object Reference") (OtherComp :type "PrimitiveComponent Object Reference") (OtherBodyIndex :type Integer) (bFromSweep :type Boolean) (SweepResult :type "HitResult Structure (by ref)"))
  (bind _trigger (`self.Trigger`))
  ;[1 1 1] Checkpoint system cleared when overlap occurs
  (bind _ashoverboard_component (cast `/Game/A_ProgrammerCommon/Blueprints/HoverboardComponent` OtherActor)) ; Check if collider is hoverboard
  (if (> (`KismetMathLibrary.Dot_VectorVector` (`SceneComponent.GetComponentVelocity` (`/Game/A_ProgrammerCommon/Blueprints/HoverboardComponent.Cube` _ashoverboard_component)) (`KismetMathLibrary.Conv_RotatorToVector` (`SceneComponent.K2_GetComponentRotation` (`self.Arrow`)))) 0.0)
    (`self.CheckpointCleared` (`self.CheckpointNumber`))
    (`SceneComponent.SetHiddenInGame` _trigger true false)
    (`SceneComponent.SetHiddenInGame` (`self.ParticleSystem`) true false)
    (set `PrimitiveComponent.bGenerateOverlapEvents` false _trigger)))

(fn `UserConstructionScript`)