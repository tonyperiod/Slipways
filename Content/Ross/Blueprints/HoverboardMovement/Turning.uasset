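; Turning component for a physics-driven hoverboard, steering it from the Move Right / Left input axis.
; InitComponent takes a hoverboard reference, casts it to HoverboardComponent, and caches its Cube body and rotation rate.
; Each axis update yaws the Cube and rotates its linear velocity by the same amount, so momentum follows the heading.
; The same scaled value is stored as TonyLean.
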(event `InitComponent`
  (params (HoverboardReference :type "/Game/A_ProgrammerCommon/Blueprints/HoverboardComponent Object Reference"))
  (bind _output_get (set `self.Hoverboard Reference` HoverboardReference))
  (bind _ashoverboard_component (cast `/Game/A_ProgrammerCommon/Blueprints/HoverboardComponent` _output_get))
  (set `self.Cube` (`/Game/A_ProgrammerCommon/Blueprints/HoverboardComponent.Cube` _ashoverboard_component))
  (set `self.Rotation Value Local` (`/Game/A_ProgrammerCommon/Blueprints/HoverboardComponent.rotationValue` _ashoverboard_component)))

(event `InputAxis|Move Right / Left`
  (params (AxisValue :type "Float (single-precision)"))
  (bind _returnvalue (* AxisValue (`self.Rotation Value Local`)))
  (bind _returnvalue_2 (`KismetMathLibrary.MakeRotator` 0.0 0.0 _returnvalue))
  (bind _returnvalue_3 (`PrimitiveComponent.GetPhysicsLinearVelocity` (`self.Cube`) "None"))
  (`PrimitiveComponent.SetPhysicsLinearVelocity` (`self.Cube`) (`KismetMathLibrary.GreaterGreater_VectorRotator` _returnvalue_3 _returnvalue_2) false "None")
  (`self.K2_AddLocalRotation` (`self.Cube`) _returnvalue_2 false false)
  ;[1 0.04373 0.8965] Tony's Stuff
  (set `self.Tony_Lean` _returnvalue))