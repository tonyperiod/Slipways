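; Checkpoint actor that updates a hoverboard's respawn location when it enters the trigger.
; On overlap it casts the other actor to HoverboardComponent and copies the SpawnPoint world transform into its SpawnPosition.
; It then reaches the HUD widget through the RacingInstance game instance and shows a "Checkpoint" message, hiding it after a short delay.
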(event `self.Trigger.OnComponentBeginOverlap`
  (params (OverlappedComponent :type "PrimitiveComponent Object Reference") (OtherActor :type "Actor Object Reference") (OtherComp :type "PrimitiveComponent Object Reference") (OtherBodyIndex :type Integer) (bFromSweep :type Boolean) (SweepResult :type "HitResult Structure (by ref)"))
  (bind _ashoverboard_component (cast `/Game/A_ProgrammerCommon/Blueprints/HoverboardComponent` OtherActor))
  (set `/Game/A_ProgrammerCommon/Blueprints/HoverboardComponent.SpawnPosition` (`SceneComponent.K2_GetComponentToWorld` (`self.SpawnPoint`)) _ashoverboard_component)
  (bind _asracing_instance (cast `/Game/Ross/Blueprints/BasicTimer/RacingInstance` (`GameplayStatics.GetGameInstance`)))
  (bind _message (`/Game/Ross/Blueprints/BasicTimer/RacingWidget.Message` (`/Game/Ross/Blueprints/BasicTimer/RacingInstance.Widget` _asracing_instance)))
  (`TextBlock.SetText` _message "Checkpoint")
  (`Widget.SetVisibility` _message "Visible")
  (`KismetSystemLibrary.Delay` 1.0)
  (`Widget.SetVisibility` _message "Hidden"))

(fn `UserConstructionScript`)