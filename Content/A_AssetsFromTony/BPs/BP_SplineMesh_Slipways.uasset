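; Spline-driven construction-script builder for a slipway track section, with optional side walls, pillars and overhead beams.
; It derives two offset wall splines from the main spline, reversing the left one's point order, then lays spline meshes per segment for track and walls.
; Instanced pillars follow the enabled walls' points, while instanced beams repeat along the main spline at intervals based on beam mesh bounds, both yaw-only.
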(fn `UserConstructionScript`
  (bind _returnvalue_x (`KismetMathLibrary.BreakVector` (`self.GetActorScale3D`)))
  (bind _r_wall_spline_pos (`self.R Wall Spline Pos`))
  (bind _trackside (`self.Trackside`))
  (bind _spline (`self.Spline`))
  (bind _spline_2 (`self.Spline`))
  (bind _instance_pillar (`self.Instance Pillar`))
  (bind _l_wall_spline_pos (`self.L Wall Spline Pos`))
  (bind _spline_wall_r (`self.Spline Wall R`))
  (bind _instance_pillar_2 (`self.Instance Pillar`))
  (bind _spline_wall_l (`self.Spline Wall L`))
  (bind _returnvalue (`SplineComponent.GetNumberOfSplinePoints` _spline_2))
  (bind (_min _max) (break `Box` (`StaticMesh.GetBoundingBox` (`self.Beam`))))
  (bind _returnvalue_2 (`AddComponent|NODE_AddSplineComponent-0`))
  (bind _output_get (set `self.Spline Wall R` _returnvalue_2))
  (`StaticMeshComponent.SetStaticMesh` (`self.Instance Pillar`) (`self.Pillar`))
  (`StaticMeshComponent.SetStaticMesh` (`self.Instance Beam`) (`self.Beam`))
  (bind _returnvalue_3 (`AddComponent|NODE_AddSplineComponent-1`))
  (bind _output_get_2 (set `self.Spline Wall L` _returnvalue_3))
  (for _index (range (+ _returnvalue 1))
    (bind _returnvalue_4 (- (- _returnvalue 1) _index))
    (bind _returnvalue_5 (`SplineComponent.GetLocationAtSplinePoint` _spline_2 _returnvalue_4 "Local"))
    ;[1 1 1] Left Side
    (`KismetArrayLibrary.Array_Add` _l_wall_spline_pos (`KismetMathLibrary.MakeVector` (.x (+ (* (* (`KismetMathLibrary.GetRightVector` (`SplineComponent.GetRotationAtSplinePoint` _spline_2 _returnvalue_4 "Local")) (-1.0 -1.0 0.0)) (`self.Walls Offset`)) _returnvalue_5)) (.y (+ (* (* (`KismetMathLibrary.GetRightVector` (`SplineComponent.GetRotationAtSplinePoint` _spline_2 _returnvalue_4 "Local")) (-1.0 -1.0 0.0)) (`self.Walls Offset`)) _returnvalue_5)) (+ (.z _returnvalue_5) (`self.Walls Vertical Offset`))))
    (bind _returnvalue_6 (`SplineComponent.GetLocationAtSplinePoint` _spline_2 _index "Local"))
    ;[1 1 1] Right Side
    (`KismetArrayLibrary.Array_Add` _r_wall_spline_pos (`KismetMathLibrary.MakeVector` (.x (+ (* (`KismetMathLibrary.GetRightVector` (`SplineComponent.GetRotationAtSplinePoint` _spline_2 _index "Local")) (`self.Walls Offset`)) _returnvalue_6)) (.y (+ (* (`KismetMathLibrary.GetRightVector` (`SplineComponent.GetRotationAtSplinePoint` _spline_2 _index "Local")) (`self.Walls Offset`)) _returnvalue_6)) (+ (.z _returnvalue_6) (`self.Walls Vertical Offset`)))))
  (`SplineComponent.SetSplinePoints` _output_get_2 _l_wall_spline_pos "Local" true)
  (`SplineComponent.SetSplinePoints` _output_get _r_wall_spline_pos "Local" true)
  (for _index_2 (range (+ (- _returnvalue 2) 1))
    (`|ExecutionSequence`
      (:`then_0`
        ;[1 1 1] Trackside L
        (if (`self.IsWallLOn`)
          (bind _returnvalue_7 (`AddComponent|NODE_AddSplineMeshComponent-2`))
          (`StaticMeshComponent.SetStaticMesh` _returnvalue_7 _trackside)
          (`PrimitiveComponent.SetCollisionEnabled` _returnvalue_7 "QueryAndPhysics")
          (bind _returnvalue_8 (+ _index_2 1))
          (`SplineMeshComponent.SetStartAndEnd` _returnvalue_7 (`SplineComponent.GetLocationAtSplinePoint` _spline_wall_l _index_2 "Local") (`SplineComponent.GetTangentAtSplinePoint` _spline_wall_l _index_2 "Local") (`SplineComponent.GetLocationAtSplinePoint` _spline_wall_l _returnvalue_8 "Local") (`SplineComponent.GetTangentAtSplinePoint` _spline_wall_l _returnvalue_8 "Local") true)
          (`SceneComponent.K2_AttachToComponent` _returnvalue_7 (`self.DefaultSceneRoot`) "None" "KeepRelative" "KeepRelative" "KeepRelative" true)))
      (:`then_1`
        ;[1 1 1] Trackside R
        (if (`self.IsWallROn`)
          (bind _returnvalue_9 (`AddComponent|NODE_AddSplineMeshComponent-1`))
          (`StaticMeshComponent.SetStaticMesh` _returnvalue_9 _trackside)
          (`PrimitiveComponent.SetCollisionEnabled` _returnvalue_9 "QueryAndPhysics")
          (bind _returnvalue_10 (+ _index_2 1))
          (`SplineMeshComponent.SetStartAndEnd` _returnvalue_9 (`SplineComponent.GetLocationAtSplinePoint` _spline_wall_r _index_2 "Local") (`SplineComponent.GetTangentAtSplinePoint` _spline_wall_r _index_2 "Local") (`SplineComponent.GetLocationAtSplinePoint` _spline_wall_r _returnvalue_10 "Local") (`SplineComponent.GetTangentAtSplinePoint` _spline_wall_r _returnvalue_10 "Local") true)
          (`SceneComponent.K2_AttachToComponent` _returnvalue_9 (`self.DefaultSceneRoot`) "None" "KeepRelative" "KeepRelative" "KeepRelative" true)))
      (:`then_2`
        ;[1 1 1] Track
        (bind _returnvalue_11 (`AddComponent|NODE_AddSplineMeshComponent-0`))
        (`StaticMeshComponent.SetStaticMesh` _returnvalue_11 (`self.splineMesh`))
        (`PrimitiveComponent.SetCollisionEnabled` _returnvalue_11 "QueryAndPhysics")
        (set `self.Tags` (`self.Tags_0`))
        (bind _returnvalue_12 (+ _index_2 1))
        (`SplineMeshComponent.SetStartAndEnd` _returnvalue_11 (`SplineComponent.GetLocationAtSplinePoint` _spline_2 _index_2 "Local") (`SplineComponent.GetTangentAtSplinePoint` _spline_2 _index_2 "Local") (`SplineComponent.GetLocationAtSplinePoint` _spline_2 _returnvalue_12 "Local") (`SplineComponent.GetTangentAtSplinePoint` _spline_2 _returnvalue_12 "Local") true)
        (`SceneComponent.K2_AttachToComponent` _returnvalue_11 (`self.DefaultSceneRoot`) "None" "KeepRelative" "KeepRelative" "KeepRelative" true))
      (:`then_3`
        ;[1 1 1] Pillars
        (if (`self.IsWallLOn`) :!label _label
          (bind _location (.location (`SplineComponent.GetTransformAtSplinePoint` (`self.Spline Wall L`) _index_2 "Local" false)))
          (bind _rotation (.rotation (`SplineComponent.GetTransformAtSplinePoint` (`self.Spline Wall L`) _index_2 "Local" false)))
          ;;[1 1 1] L Base
          (`InstancedStaticMeshComponent.AddInstance` _instance_pillar_2 (`KismetMathLibrary.MakeTransform` (`KismetMathLibrary.MakeVector` (.x (+ (* (`KismetMathLibrary.GetRightVector` _rotation) (* (`self.Pillars Offset`) -1.0)) _location)) (.y (+ (* (`KismetMathLibrary.GetRightVector` _rotation) (* (`self.Pillars Offset`) -1.0)) _location)) (+ (.z _location) (`self.Pillar Vertical Offset`))) (`KismetMathLibrary.MakeRotator` 0.0 0.0 (.yaw _rotation))) false)
          (`PrimitiveComponent.SetCollisionEnabled` _instance_pillar_2 "QueryAndPhysics")))
      (:`then_4`
        (if (`self.IsWallROn`) :!label _label_2
          (bind _location_2 (.location (`SplineComponent.GetTransformAtSplinePoint` (`self.Spline Wall R`) _index_2 "Local" false)))
          (bind _rotation_2 (.rotation (`SplineComponent.GetTransformAtSplinePoint` (`self.Spline Wall R`) _index_2 "Local" false)))
          ;;[1 1 1] R Base
          (`InstancedStaticMeshComponent.AddInstance` _instance_pillar (`KismetMathLibrary.MakeTransform` (`KismetMathLibrary.MakeVector` (.x (+ (* (`KismetMathLibrary.GetRightVector` _rotation_2) (* (`self.Pillars Offset`) -1.0)) _location_2)) (.y (+ (* (`KismetMathLibrary.GetRightVector` _rotation_2) (* (`self.Pillars Offset`) -1.0)) _location_2)) (+ (.z _location_2) (`self.Pillar Vertical Offset`))) (`KismetMathLibrary.MakeRotator` 0.0 0.0 (.yaw _rotation_2))) false)
          (`PrimitiveComponent.SetCollisionEnabled` _instance_pillar "QueryAndPhysics")))))
  (`|ExecutionSequence`
    (:`then_0`
      (goto _label))
    (:`then_1`
      (goto _label_2))
    (:`then_2`
      ;[1 1 1] Top Beams
      ;;[1 1 1] Get Asset Size and set up mesh
      (if (`self.IaBeamOn`)
        (bind _output_get_3 (set `self.Section Length Coeff` (+ (- (.x _max) (.x _min)) (`self.Beam Horizontal Offset`))))
        ;;[1 1 1] Section length = mesh Length
        (set `self.Section Length` (* _returnvalue_x _output_get_3))
        (for _index_3 (range (`KismetMathLibrary.FTrunc` (/ (`SplineComponent.GetSplineLength` (`self.Spline`)) (`self.Section Length`))))
          (bind _returnvalue_13 (* _index_3 (`self.Section Length`)))
          (bind (_x _y _z) (`KismetMathLibrary.BreakVector3f` (`SplineComponent.GetLocationAtDistanceAlongSpline` _spline _returnvalue_13 "Local")))
          (`InstancedStaticMeshComponent.AddInstance` (`self.Instance Beam`) (`KismetMathLibrary.MakeTransform` (`KismetMathLibrary.MakeVector` _x _y (+ _z (`self.Beam Vertical Offset`))) (`KismetMathLibrary.MakeRotator` 0.0 0.0 (+ (.yaw (`SplineComponent.GetRotationAtDistanceAlongSpline` _spline _returnvalue_13 "Local")) 0.0))) false))))))